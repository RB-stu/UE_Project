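; BP_WeaponsBase is a base weapon Blueprint that handles showing, hiding and attacking with a character's weapon.
; WeaponInInventory and WeaponInHand toggle visibility of the root component and its children.
; CommitAttackAnimNotify calls Attack, which checks that WeaponState is the enum's NewEnumerator0 value before playing the AttackAnim montage.
; The montage plays on the skeletal mesh of the weapon's owner, found by casting it to Character.
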(event `WeaponInInventory`
  (`SceneComponent.SetVisibility` (`self.DefaultSceneRoot`) false true))

(event `WeaponInHand`
  (`SceneComponent.SetVisibility` (`self.DefaultSceneRoot`) true true))

(event `CommitAttackAnimNotify`
  ; Attack Box
  (`self.Attack`))

(event `Attack`
  ; Attack Box
  (bind _result (`self.CanAttack`))
  (if _result
    (`self.PlayAttackAnim`)))

(event `PlayAttackAnim`
  ; Attack Box
  (`|PlayMontage` (`self.EghGetPawnSkeletalMesh`) (`self.AttackAnim`)))

(fn `CanAttack`
  (returns (Result :type Boolean))
  (return (`|EnumEquality` (`self.WeaponState`) "NewEnumerator0")))

(fn `EghGetPawnSkeletalMesh`
  (returns (Mesh :type "SkeletalMeshComponent Object Reference"))
  (bind _ascharacter (cast `Character` (`self.GetOwner`))
    (:`then`
      _)
    (:`CastFailed`
      _))
  (return (`Character.Mesh` _ascharacter)))

(fn `UserConstructionScript`)